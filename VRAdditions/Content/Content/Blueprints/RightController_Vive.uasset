(event `self.ReceiveBeginPlay`
  (bind _returnvalue (`EnhancedInputLibrary.MakeInputActionValueOfType` 1.0 0.0 0.0 "Boolean"))
  (bind _returnvalue_2 (pcsubsystem `EnhancedInputLocalPlayerSubsystem` (`GameplayStatics.GetPlayerController` 0)))
  (`self.EnableInput` (`GameplayStatics.GetPlayerController` 0))
  (`self.K2_SetActorLocation` self (+ (`self.K2_GetActorLocation` (`GameplayStatics.GetPlayerPawn` 0)) (200.0 0.0 0.0)) false false)
  (`KismetSystemLibrary.Delay` 0.2)
  (bind _asfgcharacter_player (cast `FGCharacterPlayer` (`GameplayStatics.GetPlayerCharacter` 0))
    (:`then`
      (bind _returnvalue_3 (`FGCharacterPlayer.GetBuildGun` _asfgcharacter_player))
      (add `FGBuildGun.mOnStateChanged` _returnvalue_3 (`|CreateDelegate` :!event `OnChangeBuildGunStateEvent`))
      (bind (_out_recipes _out_customizationrecipes) (`FGBuildGun.GetAvailableRecipes` _returnvalue_3))
      (set `self._CurrentRecipes` _out_recipes)
      (set `self._CurrentCustomizationRecipes` _out_customizationrecipes)
      (add `FGRecipeManager.mOnRecipeAvailable` (`FGRecipeManager.Get` _returnvalue_3) (delegate `OnRecipeChangedEvent`))
      (`KismetSystemLibrary.Delay` 1.0)
      (`EnhancedInputSubsystemInterface.InjectInputForAction` :`self` _returnvalue_2 :`Action` "/Game/FactoryGame/Inputs/Player/Actions/IA_ToggleBuildGunDismantle.IA_ToggleBuildGunDismantle" :`RawValue` _returnvalue)
      (`KismetSystemLibrary.Delay` 1.0)
      (`EnhancedInputSubsystemInterface.InjectInputForAction` :`self` _returnvalue_2 :`Action` "/Game/FactoryGame/Inputs/Player/Actions/IA_ToggleBuildGunDismantle.IA_ToggleBuildGunDismantle" :`RawValue` _returnvalue))
    (:`CastFailed`
      (`/VRAdditions/Content/UI/Widget_DebugInfo.Set Slot String` (`/VRAdditions/Content/Blueprints/VRCore.DebugInfo` (`self._VRCore`)) "VRInput_Right Log " "Cast FAILD!"))))

(event `OnRecipeChangedEvent`
  (params (recipeClass :type "FGRecipe Class Reference"))
  (`KismetArrayLibrary.Array_Add` (`self._CurrentRecipes`) recipeClass))

(event `EnhancedInput|/VRAdditions/Content/Inputs/VRInputRMenu`
  (params (ActionValue :type Boolean) (ElapsedSeconds :type "Float (double-precision)") (TriggeredSeconds :type "Float (double-precision)") (InputAction :type "InputAction Object Reference" :default "/VRAdditions/Content/Inputs/VRInputRMenu.VRInputRMenu"))
  (bind _returnvalue (`self.GetActorForwardVector` self))
  (bind _returnvalue_2 (`KismetMathLibrary.Dot_VectorVector` (`self._mPrevRight`) _returnvalue))
  (bind _returnvalue_3 (`KismetMathLibrary.Dot_VectorVector` (`self._mPrevUp`) _returnvalue))
  (bind _returnvalue_4 (`KismetMathLibrary.Hypotenuse` _returnvalue_2 _returnvalue_3))
  (bind _f (`self._YX2FloatRad` _returnvalue_3 _returnvalue_2))
  (:`Started`
    (`self.SetInputStatus` 0 true)
    ;[1 1 1] Get Dot product from Last A Vector and Current A Vector. (Controller only)
    (set `self._mPrevRight` (`self.GetActorRightVector` self))
    (set `self._mPrevUp` (`self.GetActorUpVector` self)))
  (:`Canceled`
    (`self.SetInputStatus` 0 :!label _label)
    (`/VRAdditions/Content/UI/Widget_DebugInfo.Set Slot String` (`/VRAdditions/Content/Blueprints/VRCore.DebugInfo` (`self._VRCore`)) "VRInput Log4 " (`KismetStringLibrary.Concat_StrStr` "VRInputRight Menu : " "Dis : " (`KismetStringLibrary.Conv_DoubleToString` _returnvalue_4) " Rad : " (`KismetStringLibrary.Conv_DoubleToString` _f)))
    (`self.MenuCalc` _f _returnvalue_4))
  (:`Completed`
    (goto _label)))

(event `self.ReceiveTick`
  (params (DeltaSeconds :type "Float (single-precision)"))
  (bind (_x _y) (`KismetMathLibrary.BreakVector2D` (`|GetInputActionValue`)))
  (bind _returnvalue (`KismetMathLibrary.Hypotenuse` _x _y))
  (`|ExecutionSequence`
    (:`then_0`
      (if (and (`|GetArrayItem` (`self._mInputStatus`) 1) (> _returnvalue 0.2))
        (`self.PadCalc` DeltaSeconds _returnvalue)))
    (:`then_1`
      (if (and (< _returnvalue 0.2) (`|GetArrayItem` (`self._mInputStatus`) 2))
        (`EnhancedInputSubsystemInterface.InjectInputForAction` :`self` (pcsubsystem `EnhancedInputLocalPlayerSubsystem` (`GameplayStatics.GetPlayerController` 0)) :`Action` "/Game/FactoryGame/Inputs/Player/Movement/IA_Crouch.IA_Crouch" :`RawValue` (`EnhancedInputLibrary.MakeInputActionValueOfType` 1.0 0.0 0.0 "Boolean"))))
    (:`then_2`
      (`self.TriggerCalc`))))

(event `EnhancedInput|/VRAdditions/Content/Inputs/VRInputRPad`
  (params (ActionValue :type "Vector2D Structure") (ElapsedSeconds :type "Float (double-precision)") (TriggeredSeconds :type "Float (double-precision)") (InputAction :type "InputAction Object Reference" :default "/VRAdditions/Content/Inputs/VRInputRPad.VRInputRPad"))
  (:`Started`
    (`self.SetInputStatus` 1 true))
  (:`Canceled`
    (`self.SetInputStatus` 1 :!label _label_2))
  (:`Completed`
    (goto _label_2)))

(event `EnhancedInput|/VRAdditions/Content/Inputs/VRInputRPadClick`
  (params (ActionValue :type Boolean) (ElapsedSeconds :type "Float (double-precision)") (TriggeredSeconds :type "Float (double-precision)") (InputAction :type "InputAction Object Reference" :default "/VRAdditions/Content/Inputs/VRInputRPadClick.VRInputRPadClick"))
  (:`Started`
    (`self.SetInputStatus` 2 true))
  (:`Canceled`
    (`self.SetInputStatus` 2 :!label _label_3)
    (`self.SetInputStatus` 3))
  (:`Completed`
    (goto _label_3)))

(event `EnhancedInput|/VRAdditions/Content/Inputs/VRInputRGrip`
  (params (ActionValue :type Boolean) (ElapsedSeconds :type "Float (double-precision)") (TriggeredSeconds :type "Float (double-precision)") (InputAction :type "InputAction Object Reference" :default "/VRAdditions/Content/Inputs/VRInputRGrip.VRInputRGrip"))
  (:`Started`
    (`self.SetInputStatus` 4 true)
    (if ActionValue
      (`EnhancedInputSubsystemInterface.InjectInputForAction` :`self` (pcsubsystem `EnhancedInputLocalPlayerSubsystem` (`GameplayStatics.GetPlayerController` 0)) :`Action` "/Game/FactoryGame/Inputs/Player/Actions/IA_BuildingSample.IA_BuildingSample" :`RawValue` (`EnhancedInputLibrary.MakeInputActionValueOfType` 1.0 0.0 0.0 "Boolean"))))
  (:`Canceled`
    (`self.SetInputStatus` 4 :!label _label_4))
  (:`Completed`
    (goto _label_4)))

(event `EnhancedInput|/VRAdditions/Content/Inputs/VRInputRTrigger`
  (params (ActionValue :type Boolean) (ElapsedSeconds :type "Float (double-precision)") (TriggeredSeconds :type "Float (double-precision)") (InputAction :type "InputAction Object Reference" :default "/VRAdditions/Content/Inputs/VRInputRTrigger.VRInputRTrigger"))
  (:`Started`
    (`self.SetInputStatus` 5 true)
    (`self.TriggerOnceCalc`))
  (:`Canceled`
    (`self.SetInputStatus` 5 :!label _label_5))
  (:`Completed`
    (goto _label_5)))

(event `OnChangeBuildGunStateEvent`
  (params (newState :type "EBuildGunState Enum" :default "BGS_NONE"))
  (bind __rcurrentstate (`self._RCurrentState`))
  (bind __leftcontroller (`self._LeftController`))
  (`/VRAdditions/Content/UI/Widget_DebugInfo.Set Slot String` (`/VRAdditions/Content/Blueprints/VRCore.DebugInfo` (`self._VRCore`)) "VRInput_Right Log2 " (`KismetStringLibrary.Concat_StrStr` "OnBuildGunState Changed : " (`|GetEnumeratorNameAsString` newState)))
  (switch `EBuildGunState` newState
    (:`BGS_NONE`
      (if (not (or (`|EnumEquality` __rcurrentstate "NewEnumerator6") (`|EnumEquality` __rcurrentstate "NewEnumerator7") (`|EnumEquality` __rcurrentstate "NewEnumerator9")))
        (`self.ChangeState` "NewEnumerator0")
        (`/VRAdditions/Content/Blueprints/LeftController_Vive.ChangeState` __leftcontroller "NewEnumerator0")))
    (:`BGS_BUILD`
      (`self.ChangeState` "NewEnumerator1")
      (`/VRAdditions/Content/Blueprints/LeftController_Vive.ChangeState` __leftcontroller "NewEnumerator1")
      (set `self._mIsNudging` false))
    (:`BGS_DISMANTLE`
      (`self.ChangeState` "NewEnumerator2")
      (`/VRAdditions/Content/Blueprints/LeftController_Vive.ChangeState` __leftcontroller "NewEnumerator2"))
    (:`BGS_PAINT`
      (`self.ChangeState` "NewEnumerator3")
      (`/VRAdditions/Content/Blueprints/LeftController_Vive.ChangeState` __leftcontroller "NewEnumerator3"))))

(event `OnChangeStateExit_Event`
  (params (`Exit State` :type "/VRAdditions/Content/Blueprints/VRControllerStates Enum (by ref)"))
  (switch `/VRAdditions/Content/Blueprints/VRControllerStates` `Exit State`
    (:`NewEnumerator6`
      _)
    (:`NewEnumerator7`
      _)
    (:`NewEnumerator9`
      _))
  (`/VRAdditions/Content/Blueprints/VRCore.OpenCloseMenu` (`self._VRCore`) "NewEnumerator0"))

(event `OnChangeStatePre_Event`
  (params (`In State` :type "/VRAdditions/Content/Blueprints/VRControllerStates Enum (by ref)"))
  (bind __vrcore (`self._VRCore`))
  (`/VRAdditions/Content/UI/Widget_DebugInfo.Set Slot String` (`/VRAdditions/Content/Blueprints/VRCore.DebugInfo` (`self._VRCore`)) "VRInput_Right Log State" (`KismetStringLibrary.Concat_StrStr` "Pre called! with " (`|GetEnumeratorNameAsString` `In State`)))
  (switch `/VRAdditions/Content/Blueprints/VRControllerStates` `In State`
    (:`NewEnumerator6`
      (`/VRAdditions/Content/Blueprints/VRCore.OpenCloseMenu` __vrcore "NewEnumerator1"))
    (:`NewEnumerator7`
      (`/VRAdditions/Content/Blueprints/VRCore.OpenCloseMenu` __vrcore "NewEnumerator2"))
    (:`NewEnumerator9`
      (`/VRAdditions/Content/Blueprints/VRCore.OpenCloseMenu` __vrcore "NewEnumerator3"))))

(fn `_Timer`
  (params (_DeltaTime :type "Float (double-precision)") (Threshold :type "Float (double-precision)"))
  (returns (Ticked :type Boolean))
  (bind _output_get (set `self._mPrevTime` (+ (`self._mPrevTime`) _DeltaTime)))
  (if (> _output_get Threshold)
    (set `self._mPrevTime` 0.0)
    (return true)
    (else
      (return false))))

(fn `ChangeState`
  (params (NewState :type "/VRAdditions/Content/Blueprints/VRControllerStates Enum" :default "NewEnumerator0"))
  (bind __rcurrentstate (`self._RCurrentState`))
  (if (`|EnumEquality` __rcurrentstate NewState)
    (return)
    (else
      (`self.OnChangeStateExit_Event` __rcurrentstate)
      (bind _output_get (set `self._RCurrentState` NewState))
      (`self.OnChangeStatePre_Event` _output_get)
      (return))))

(fn `MenuCalc`
  (params (RadFloat :type "Float (double-precision)") (Hypotenuse :type "Float (double-precision)"))
  (bind __leftcontroller (`self._LeftController`))
  (switch `/VRAdditions/Content/Blueprints/VRControllerStates` (`self._RCurrentState`)
    (:`NewEnumerator0`
      (if (and (> RadFloat 0.25) (< RadFloat 0.75))
        (`self.ChangeState` "NewEnumerator6")
        (`/VRAdditions/Content/Blueprints/LeftController_Vive.ChangeState` __leftcontroller "NewEnumerator6")
        (elif (and (> RadFloat 0.75) (< RadFloat 1.25))
          (`self.ChangeState` "NewEnumerator7")
          (`/VRAdditions/Content/Blueprints/LeftController_Vive.ChangeState` __leftcontroller "NewEnumerator7")
          (elif (and (> RadFloat 1.25) (< RadFloat 1.75))
            (`self.ChangeState` "NewEnumerator2")
            (`/VRAdditions/Content/Blueprints/LeftController_Vive.ChangeState` __leftcontroller "NewEnumerator2")
            (bind _asfgcharacter_player (cast `FGCharacterPlayer` (`GameplayStatics.GetPlayerCharacter` 0)))
            (`FGCharacterPlayer.HotKeyDismantle` _asfgcharacter_player)
            (elif (or (< RadFloat 0.25) (> RadFloat 1.75))
              (`self.ChangeState` "NewEnumerator9")
              (`/VRAdditions/Content/Blueprints/LeftController_Vive.ChangeState` __leftcontroller "NewEnumerator9"))))))))

(fn `PadCalc`
  (params (DeltaTime :type "Float (single-precision)") (Hypoteuse :type "Float (double-precision)"))
  (bind __minputstatus (`self._mInputStatus`))
  (bind (_x _y) (`KismetMathLibrary.BreakVector2D` (`|GetInputActionValue`)))
  (bind _returnvalue (pcsubsystem `EnhancedInputLocalPlayerSubsystem` (`GameplayStatics.GetPlayerController` 0)))
  (bind _debuginfo (`/VRAdditions/Content/Blueprints/VRCore.DebugInfo` (`self._VRCore`)))
  (bind _f (`self._YX2FloatRad` _y _x))
  ;[1 1 1] Check Right Touched
  (if (or (< _f 0.125) (> _f 1.875))
    (switch `/VRAdditions/Content/Blueprints/VRControllerStates` (`self._RCurrentState`)
      (:`NewEnumerator0`
        (`EnhancedInputSubsystemInterface.InjectInputForAction` :`self` _returnvalue :`Action` "/Game/FactoryGame/Inputs/Player/Movement/IA_LookAxis.IA_LookAxis" :`RawValue` (`EnhancedInputLibrary.MakeInputActionValueOfType` (* DeltaTime 20.0) 0.0 0.0 "Axis2D") :!label _label))
      (:`NewEnumerator1`
        (goto _label))
      (:`NewEnumerator2`
        (goto _label))
      (:`NewEnumerator3`
        (goto _label))
      (:`NewEnumerator4`
        (goto _label))
      (:`NewEnumerator6`
        (bind _ticked (`self._Timer` DeltaTime 0.12))
        (if _ticked
          (bind _result (`/Engine/EditorBlueprintResources/StandardMacros.IncrementInt` (`self._CurrentSelectedRecipeID`))
            (:`  `
              (if (>= _result (`KismetArrayLibrary.Array_Length` (`self._CurrentRecipes`)))
                (set `self._CurrentSelectedRecipeID` 0))
              (`self.OnChangeSelectingRecipe`)
              (`/VRAdditions/Content/UI/Widget_DebugInfo.Set Slot String` _debuginfo "VRInput_Right Log Select Recipe" "Right Called!"))))))
    (else
      ;[1 1 1] Check Left Touched
      (if (and (> _f 0.875) (< _f 1.125))
        (switch `/VRAdditions/Content/Blueprints/VRControllerStates` (`self._RCurrentState`)
          (:`NewEnumerator0`
            (`EnhancedInputSubsystemInterface.InjectInputForAction` :`self` _returnvalue :`Action` "/Game/FactoryGame/Inputs/Player/Movement/IA_LookAxis.IA_LookAxis" :`RawValue` (`EnhancedInputLibrary.MakeInputActionValueOfType` (* DeltaTime -20.0) 0.0 0.0 "Axis2D") :!label _label_2))
          (:`NewEnumerator1`
            (goto _label_2))
          (:`NewEnumerator2`
            (goto _label_2))
          (:`NewEnumerator3`
            (goto _label_2))
          (:`NewEnumerator4`
            (goto _label_2))
          (:`NewEnumerator6`
            (bind _ticked_2 (`self._Timer` DeltaTime 0.12))
            (if _ticked_2
              (bind _result_2 (`/Engine/EditorBlueprintResources/StandardMacros.DecrementInt` (`self._CurrentSelectedRecipeID`))
                (:`  `
                  (if (< _result_2 0)
                    (set `self._CurrentSelectedRecipeID` (- (`KismetArrayLibrary.Array_Length` (`self._CurrentRecipes`)) 1)))
                  (`self.OnChangeSelectingRecipe`)
                  (`/VRAdditions/Content/UI/Widget_DebugInfo.Set Slot String` _debuginfo "VRInput_Right Log Select Recipe" "Left Called!"))))))
        (else
          ;[1 1 1] Check Down Touched
          (if (and (> _f 0.125) (< _f 0.875))
            (switch `/VRAdditions/Content/Blueprints/VRControllerStates` (`self._RCurrentState`)
              (:`NewEnumerator1`
                (if (`self._mIsNudging`)
                  (`EnhancedInputSubsystemInterface.InjectInputForAction` :`self` _returnvalue :`Action` "/Game/FactoryGame/Inputs/Equipment/Buildgun/Build/IA_HologramNudgeAxis.IA_HologramNudgeAxis" :`RawValue` (`EnhancedInputLibrary.MakeInputActionValueOfType` -1.0 0.0 0.0 "Axis2D"))
                  (else
                    (bind _ticked_3 (`self._Timer` DeltaTime 0.2))
                    (if _ticked_3
                      (`EnhancedInputSubsystemInterface.InjectInputForAction` :`self` _returnvalue :`Action` "/Game/FactoryGame/Inputs/Equipment/IA_Scroll.IA_Scroll" :`RawValue` (`EnhancedInputLibrary.MakeInputActionValueOfType` -1.0 0.0 0.0 "Axis1D")))))))
            (else
              ;[1 1 1] Check Top Touched
              (if (and (> _f 1.125) (< _f 1.875))
                (switch `/VRAdditions/Content/Blueprints/VRControllerStates` (`self._RCurrentState`)
                  (:`NewEnumerator0`
                    ;[1 1 1] Ping
                    (if (and (not (`|GetArrayItem` __minputstatus 3)) (`|GetArrayItem` __minputstatus 2) (> Hypoteuse 0.2))
                      (`self.SetInputStatus` 3 true)
                      (`EnhancedInputSubsystemInterface.InjectInputForAction` :`self` _returnvalue :`Action` "/Game/FactoryGame/Inputs/Player/ControllerActions/IA_AttentionPing.IA_AttentionPing" :`RawValue` (`EnhancedInputLibrary.MakeInputActionValueOfType` 1.0 0.0 0.0 "Boolean"))))
                  (:`NewEnumerator1`
                    (if (`self._mIsNudging`)
                      (`EnhancedInputSubsystemInterface.InjectInputForAction` :`self` _returnvalue :`Action` "/Game/FactoryGame/Inputs/Equipment/Buildgun/Build/IA_HologramNudgeAxis.IA_HologramNudgeAxis" :`RawValue` (`EnhancedInputLibrary.MakeInputActionValueOfType` 1.0 0.0 0.0 "Axis2D"))
                      (else
                        (bind _ticked_4 (`self._Timer` DeltaTime 0.2))
                        (if _ticked_4
                          (`EnhancedInputSubsystemInterface.InjectInputForAction` :`self` _returnvalue :`Action` "/Game/FactoryGame/Inputs/Equipment/IA_Scroll.IA_Scroll" :`RawValue` (`EnhancedInputLibrary.MakeInputActionValueOfType` 1.0 0.0 0.0 "Axis1D")))))))))))))))

(fn `SetInputStatus`
  (params (Index :type Integer) (Value :type Boolean))
  (`KismetArrayLibrary.Array_Set` (`self._mInputStatus`) Index Value))

(fn `TriggerCalc`
  (if (`|GetArrayItem` (`self._mInputStatus`) 5)
    (switch `/VRAdditions/Content/Blueprints/VRControllerStates` (`self._RCurrentState`)
      (:`NewEnumerator2`
        (`EnhancedInputSubsystemInterface.InjectInputForAction` :`self` (pcsubsystem `EnhancedInputLocalPlayerSubsystem` (`GameplayStatics.GetPlayerController` 0)) :`Action` "/Game/FactoryGame/Inputs/Equipment/Buildgun/IA_BuildGun_PrimaryFire.IA_BuildGun_PrimaryFire" :`RawValue` (`EnhancedInputLibrary.MakeInputActionValueOfType` 1.0 0.0 0.0 "Boolean"))))))

(fn `TriggerOnceCalc`
  (switch `/VRAdditions/Content/Blueprints/VRControllerStates` (`self._RCurrentState`)
    (:`NewEnumerator1`
      (`EnhancedInputSubsystemInterface.InjectInputForAction` :`self` (pcsubsystem `EnhancedInputLocalPlayerSubsystem` (`GameplayStatics.GetPlayerController` 0)) :`Action` "/Game/FactoryGame/Inputs/Equipment/Buildgun/Build/IA_HologramLock.IA_HologramLock" :`RawValue` (`EnhancedInputLibrary.MakeInputActionValueOfType` 1.0 0.0 0.0 "Boolean"))
      (set `self._mIsNudging` (not (`self._mIsNudging`))))
    (:`NewEnumerator6`
      (`self.ChangeState` "NewEnumerator1")
      (`/VRAdditions/Content/Blueprints/LeftController_Vive.ChangeState` (`self._LeftController`) "NewEnumerator1")
      (bind _asfgcharacter_player (cast `FGCharacterPlayer` (`GameplayStatics.GetPlayerCharacter` 0)))
      (`FGCharacterPlayer.HotKeyRecipe` _asfgcharacter_player (`|GetArrayItem` (`self._CurrentRecipes`) (`self._CurrentSelectedRecipeID`))))))

(fn `UserConstructionScript`)