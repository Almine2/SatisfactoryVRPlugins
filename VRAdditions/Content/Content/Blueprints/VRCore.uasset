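; VRCore is the central actor of a VR addon, setting up Vive motion controllers and floating in-world menus.
; After a startup delay it spawns cross-linked controllers and two widget floaters at the player pawn, registers references with VRAdditions_Subsystem and adds a debug HUD.
; OpenCloseMenu routes building, paint and blueprint selectors to the first floater and machine UI to the larger second.
; Tick keeps the HUD crosshair hidden.
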(event `self.ReceiveBeginPlay`
  (bind _returnvalue (`self.K2_GetActorLocation` (`GameplayStatics.GetPlayerPawn` 0)))
  (bind _returnvalue_2 (`KismetMathLibrary.MakeTransform` (+ _returnvalue (5.0 0.0 0.0))))
  (`KismetSystemLibrary.Delay` 2.0)
  (`self.K2_SetActorLocation` _returnvalue)
  (bind _returnvalue_3 (`|SpawnActorFromClass` "/VRAdditions/Content/Blueprints/LeftController_Vive.LeftController_Vive_C" (`KismetMathLibrary.MakeTransform` _returnvalue) "AlwaysSpawn" "MultiplyWithRoot" null null))
  (set `/VRAdditions/Content/Blueprints/LeftController_Vive._VRCore` self _returnvalue_3)
  (set `self.LeftController` _returnvalue_3)
  (bind _returnvalue_4 (`|SpawnActorFromClass` "/VRAdditions/Content/Blueprints/RightController_Vive.RightController_Vive_C" _returnvalue_2 "AlwaysSpawn" "MultiplyWithRoot" null null))
  (set `/VRAdditions/Content/Blueprints/LeftController_Vive._RightController` _returnvalue_4 _returnvalue_3)
  (set `/VRAdditions/Content/Blueprints/RightController_Vive._VRCore` self _returnvalue_4)
  (set `/VRAdditions/Content/Blueprints/RightController_Vive._LeftController` _returnvalue_3 _returnvalue_4)
  (set `self.RightController` _returnvalue_4)
  (bind _returnvalue_5 (`|SpawnActorFromClass` "/VRAdditions/Content/Blueprints/UI/WidgetFloater_VRAddition.WidgetFloater_VRAddition_C" _returnvalue_2 "AlwaysSpawn" "MultiplyWithRoot" self null))
  (set `self.FloatingWidget1` _returnvalue_5)
  (bind _returnvalue_6 (`|SpawnActorFromClass` "/VRAdditions/Content/Blueprints/UI/WidgetFloater_VRAddition.WidgetFloater_VRAddition_C" _returnvalue_2 "AlwaysSpawn" "MultiplyWithRoot" self null))
  (set `self.FloatingWidget2` _returnvalue_6)
  (`/VRAdditions/Content/Blueprints/UI/WidgetFloater_VRAddition.ChangeWidgetPixelSize` _returnvalue_6 (1920.0 1080.0))
  (`/VRAdditions/Content/Blueprints/UI/WidgetFloater_VRAddition.SetWidgetScale` _returnvalue_6 (1.0 1.0 1.0))
  (`/VRAdditions/VRAdditions_Subsystem.SetReferences_Vive` (`SubsystemActorManager.K2_GetSubsystemActor` (subsystem `SubsystemActorManager`) "/VRAdditions/VRAdditions_Subsystem.VRAdditions_Subsystem_C") (`self.LeftController`) (`self.RightController`) self)
  (`BlueprintLoggingLibrary.LogDisplay` "VRaddon Begin play!")
  ;[0.5294 0.7827 1] Debug widget
  (bind _returnvalue_7 (`|CreateWidget` "/VRAdditions/Content/UI/Widget_DebugHUD.Widget_DebugHUD_C"))
  (`UserWidget.AddToViewport` _returnvalue_7 0)
  (set `self.DebugInfo` (`/VRAdditions/Content/UI/Widget_DebugHUD.DebugInfo` _returnvalue_7)))

(event `self.ReceiveTick`
  (params (DeltaSeconds :type "Float (single-precision)"))
  (bind _asfghud (`/Game/FactoryGame/Interface/UI/HUDHelpers/BPHUDHelpers.GetFGHud` (`GameplayStatics.GetPlayerController` 0)))
  (`FGHUD.SetShowCrossHair` _asfghud false))

(fn `OpenCloseMenu`
  (params (Open :type "/VRAdditions/Content/Blueprints/VRUIMenu Enum" :default "NewEnumerator0") (MInteractObject :type "Actor Object Reference"))
  (bind _floatingwidget2 (`self.FloatingWidget2`))
  (bind _debuginfo (`self.DebugInfo`))
  (bind _rightcontroller (`self.RightController`))
  (bind _floatingwidget1 (`self.FloatingWidget1`))
  (switch `/VRAdditions/Content/Blueprints/VRUIMenu` Open
    (:`NewEnumerator0`
      (`/VRAdditions/Content/Blueprints/UI/WidgetFloater_VRAddition.Init` _floatingwidget1 0 "NewEnumerator0" null)
      (`/VRAdditions/Content/Blueprints/UI/WidgetFloater_VRAddition.Init` _floatingwidget2 0 "NewEnumerator0" null)
      (`/VRAdditions/Content/UI/Widget_DebugInfo.Set Slot String` _debuginfo "VRCore widget : " "Widget None builded?"))
    (:`NewEnumerator1`
      (`/VRAdditions/Content/Blueprints/UI/WidgetFloater_VRAddition.Init` _floatingwidget1 1 "NewEnumerator1" _rightcontroller)
      (`/VRAdditions/Content/UI/Widget_DebugInfo.Set Slot String` _debuginfo "VRCore widget : " "Widget building builded?"))
    (:`NewEnumerator2`
      (`/VRAdditions/Content/Blueprints/UI/WidgetFloater_VRAddition.Init` _floatingwidget1 1 "NewEnumerator2" _rightcontroller)
      (`/VRAdditions/Content/UI/Widget_DebugInfo.Set Slot String` _debuginfo "VRCore widget : " "Widget paint builded?"))
    (:`NewEnumerator3`
      (`/VRAdditions/Content/Blueprints/UI/WidgetFloater_VRAddition.Init` _floatingwidget1 1 "NewEnumerator3" _rightcontroller)
      (`/VRAdditions/Content/UI/Widget_DebugInfo.Set Slot String` _debuginfo "VRCore widget : " "Widget blueprint builded?"))
    (:`NewEnumerator8`
      (`/VRAdditions/Content/Blueprints/UI/WidgetFloater_VRAddition.Init` _floatingwidget2 0 "NewEnumerator8" MInteractObject)
      (`/VRAdditions/Content/UI/Widget_DebugInfo.Set Slot String` _debuginfo "VRCore widget : " "Widget MachineUI builded?"))))

(fn `UserConstructionScript`)