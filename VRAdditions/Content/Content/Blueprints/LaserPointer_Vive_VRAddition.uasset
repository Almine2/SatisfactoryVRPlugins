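; Laser pointer Blueprint, named for Vive VR, that draws a visible beam between two world points.
; OnPoint places PointerEnd at the end point and PointerMiddle at the midpoint, rotated to look from start to end.
; It scales PointerMiddle along X by the distance, keeping a thin cross-section, so one component stretches into the beam.
; The event graph and construction script hold no active logic.
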(fn `OnPoint`
  (params (End :type "Vector Structure") (Start :type "Vector Structure"))
  (bind _pointermiddle (`self.PointerMiddle`))
  (`SceneComponent.K2_SetWorldLocation` (`self.PointerEnd`) End false false)
  (`SceneComponent.K2_SetWorldLocationAndRotation` _pointermiddle (+ Start (/ (- End Start) 2.0)) (`KismetMathLibrary.FindLookAtRotation` Start End) false false)
  (`SceneComponent.SetRelativeScale3D` _pointermiddle (`KismetMathLibrary.MakeVector` (/ (`KismetMathLibrary.Vector_Distance` Start End) 100.0) 0.02 0.02)))

(fn `UserConstructionScript`)